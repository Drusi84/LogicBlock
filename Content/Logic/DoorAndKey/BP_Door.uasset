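; BP_Door is a locked door that opens when the player overlaps its Box with at least five coins while the door's HasKey flag is set.
; Opening sets IsOpening and plays a Timeline whose Update repeatedly calls MoveComponentTo, sending the Cube to a fixed raised, rotated pose.
; Debug strings report whether the door is open or closed, and nothing here closes it again.
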(event `self.Box.OnComponentBeginOverlap`
  (params (OverlappedComponent :type "PrimitiveComponent Object Reference") (OtherActor :type "Actor Object Reference") (OtherComp :type "PrimitiveComponent Object Reference") (OtherBodyIndex :type Integer) (bFromSweep :type Boolean) (SweepResult :type "HitResult Structure (by ref)"))
  (bind _asplayer (cast `/Game/Logic/DoorAndKey/Player` OtherActor))
  (if (and (>= (`/Game/Logic/DoorAndKey/Player.CoinAmount` _asplayer) 5) (`self.bHasKey`))
    (set `self.bIsOpening` true)
    (`Timeline|Timeline`
      (:`Update`
        (`KismetSystemLibrary.MoveComponentTo` (`self.Cube`) (0.0 0.0 90.0) (struct :`Roll` -90.0) false false 1.0)
        (`KismetSystemLibrary.PrintString` "Door Open")))
    (else
      (`KismetSystemLibrary.PrintString` "Door Closed"))))

(fn `UserConstructionScript`)