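; BP_KeyAndDoor is a single actor holding key and coin pickups plus the door they unlock.
; Key and coin overlaps increment counters on the BP_UIManager HUD, refresh its display and destroy the pickup component.
; The door overlap destroys the door once those HUD counts meet coin and key thresholds.
; Its coin check reuses the manager reference fetched in the coin overlap event.
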(event `self.KeyColl.OnComponentBeginOverlap`
  (params (OverlappedComponent :type "PrimitiveComponent Object Reference") (OtherActor :type "Actor Object Reference") (OtherComp :type "PrimitiveComponent Object Reference") (OtherBodyIndex :type Integer) (bFromSweep :type Boolean) (SweepResult :type "HitResult Structure (by ref)"))
  (bind _returnvalue (`GameplayStatics.GetActorOfClass` "/Game/Logic/BP_UIManager.BP_UIManager_C"))
  (bind _hud (`/Game/Logic/BP_UIManager.HUD` _returnvalue))
  (set `/Game/Logic/WBP_GameplayUI.KeyAmount` (+ (`/Game/Logic/WBP_GameplayUI.KeyAmount` _hud) 1) _hud)
  (`/Game/Logic/WBP_GameplayUI.RefreshKey` _hud)
  (`ActorComponent.K2_DestroyComponent` (`self.Key`)))

(event `self.CoinColl.OnComponentBeginOverlap`
  (params (OverlappedComponent :type "PrimitiveComponent Object Reference") (OtherActor :type "Actor Object Reference") (OtherComp :type "PrimitiveComponent Object Reference") (OtherBodyIndex :type Integer) (bFromSweep :type Boolean) (SweepResult :type "HitResult Structure (by ref)"))
  (bind _returnvalue (`GameplayStatics.GetActorOfClass` "/Game/Logic/BP_UIManager.BP_UIManager_C"))
  (bind _hud (`/Game/Logic/BP_UIManager.HUD` _returnvalue))
  (set `/Game/Logic/WBP_GameplayUI.CoinAmount` (+ (`/Game/Logic/WBP_GameplayUI.CoinAmount` _hud) 1) _hud)
  (`/Game/Logic/WBP_GameplayUI.RefreshCoin` _hud)
  (`ActorComponent.K2_DestroyComponent` (`self.Coin`)))

(event `self.DoorColl.OnComponentBeginOverlap`
  (params (OverlappedComponent :type "PrimitiveComponent Object Reference") (OtherActor :type "Actor Object Reference") (OtherComp :type "PrimitiveComponent Object Reference") (OtherBodyIndex :type Integer) (bFromSweep :type Boolean) (SweepResult :type "HitResult Structure (by ref)"))
  (bind _returnvalue (`GameplayStatics.GetActorOfClass` "/Game/Logic/BP_UIManager.BP_UIManager_C"))
  (if (and (>= (`/Game/Logic/WBP_GameplayUI.CoinAmount` (`/Game/Logic/BP_UIManager.HUD` (stale `self.CoinColl.OnComponentBeginOverlap` _returnvalue))) 5) (>= (`/Game/Logic/WBP_GameplayUI.KeyAmount` (`/Game/Logic/BP_UIManager.HUD` _returnvalue)) 1))
    (`ActorComponent.K2_DestroyComponent` (`self.Door`))))

(fn `UserConstructionScript`)