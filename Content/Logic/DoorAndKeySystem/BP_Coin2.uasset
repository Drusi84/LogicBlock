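; BP_Coin2 is a coin Blueprint in the door and key system folder that comes in Gold, Silver or Bronze variants.
; Its Construction Script uses CoinType to select the Coin variable before calling the parent Construction Script, so the parent runs with that choice already set.
; It then sets Value from the matching per-type value variable.
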(fn `UserConstructionScript`
  (locals (_GoldValue :type Integer :default 10) (_SilverValue :type Integer :default 5) (_BronzeValue :type Integer :default 1))
  (bind _cointype (`self.CoinType`))
  (set `self.Coin` (select `/Game/Logic/DoorAndKeySystem/E_CoinType` _cointype :`NewEnumerator0` (`self.Gold`) :`NewEnumerator1` (`self.Silver`) :`NewEnumerator2` (`self.Bronze`)))
  (`parent.UserConstructionScript`)
  (set `self.Value` (select `/Game/Logic/DoorAndKeySystem/E_CoinType` _cointype :`NewEnumerator0` (`local._GoldValue`) :`NewEnumerator1` (`local._SilverValue`) :`NewEnumerator2` (`local._BronzeValue`))))