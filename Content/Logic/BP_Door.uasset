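; BP_Door is a key-locked door that swings open when something overlaps its trigger box.
; The Box overlap sets IsOpening if the door's HasKey flag is true, with no check on which actor entered.
; While IsOpening is set, Tick eases the Cube's relative rotation toward a 90-degree target with RInterpTo.
; Nothing here sets HasKey or resets IsOpening, and debug strings report each state.
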(event `self.ReceiveTick`
  (params (DeltaSeconds :type "Float (single-precision)"))
  (if (stale `self.Box.OnComponentBeginOverlap` _output_get)
    (bind _output_get (set `self.TargetRotation` (struct :`Yaw` 90.0)))
    (`SceneComponent.K2_SetRelativeRotation` (`self.Cube`) (`KismetMathLibrary.RInterpTo` (`SceneComponent.RelativeRotation` (`self.Cube`)) _output_get (`GameplayStatics.GetWorldDeltaSeconds`) 5.0) false false)
    (`KismetSystemLibrary.PrintString` "Door Open")))

(event `self.Box.OnComponentBeginOverlap`
  (params (OverlappedComponent :type "PrimitiveComponent Object Reference") (OtherActor :type "Actor Object Reference") (OtherComp :type "PrimitiveComponent Object Reference") (OtherBodyIndex :type Integer) (bFromSweep :type Boolean) (SweepResult :type "HitResult Structure (by ref)"))
  (`KismetSystemLibrary.PrintString` "Door Detected")
  (if (`self.bHasKey`)
    (bind _output_get (set `self.bIsOpening` true))
    (else
      (`KismetSystemLibrary.PrintString` "Door Closed"))))

(fn `UserConstructionScript`)