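; BP_Camera is a standalone camera actor that becomes the player's view and follows the third-person character along a single axis.
; On BeginPlay it sets itself as player controller 0's view target and caches the BP_ThirdPersonCharacter found in the level.
; Each Tick it eases its world Y toward the character's with FInterpTo, keeping X and Z fixed for a smoothed side-tracking view.
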(event `self.ReceiveBeginPlay`
  (`PlayerController.SetViewTargetWithBlend` (`GameplayStatics.GetPlayerController` 0) self 0.0 "VTBlend_Linear" 0.0 false)
  (bind _returnvalue (`GameplayStatics.GetActorOfClass` "/Game/ThirdPerson/Blueprints/BP_ThirdPersonCharacter.BP_ThirdPersonCharacter_C"))
  (set `self.Player` _returnvalue))

(event `self.ReceiveTick`
  (params (DeltaSeconds :type "Float (single-precision)"))
  (bind (_returnvalue_x _returnvalue_y _returnvalue_z) (`KismetMathLibrary.BreakVector` (`self.K2_GetActorLocation`)))
  (bind (_returnvalue_x_2 _returnvalue_y_2) (`KismetMathLibrary.BreakVector` (`self.K2_GetActorLocation` (`self.Player`))))
  (`self.K2_SetActorLocation` (`KismetMathLibrary.MakeVector` _returnvalue_x (`KismetMathLibrary.FInterpTo` _returnvalue_y _returnvalue_y_2 (`GameplayStatics.GetWorldDeltaSeconds`) 2.0) _returnvalue_z)))

(fn `UserConstructionScript`)