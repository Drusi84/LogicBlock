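; A key-and-door Blueprint actor that blocks passage until the player picks up its key.
; Overlapping the key collision sets an Open flag, destroys the key component and turns the spotlight green.
; Overlapping the door collision destroys the door if Open is set, otherwise prints a "Key required" message.
; Neither overlap checks which actor triggered it.
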(event `self.KeyColl.OnComponentBeginOverlap`
  (params (OverlappedComponent :type "PrimitiveComponent Object Reference") (OtherActor :type "Actor Object Reference") (OtherComp :type "PrimitiveComponent Object Reference") (OtherBodyIndex :type Integer) (bFromSweep :type Boolean) (SweepResult :type "HitResult Structure (by ref)"))
  (set `self.Open` true)
  (`ActorComponent.K2_DestroyComponent` (`self.Key`))
  (`LightComponent.SetLightColor` (`self.SpotLight`) (make `LinearColor` 0.0 1.0) true))

(event `self.DoorColl.OnComponentBeginOverlap`
  (params (OverlappedComponent :type "PrimitiveComponent Object Reference") (OtherActor :type "Actor Object Reference") (OtherComp :type "PrimitiveComponent Object Reference") (OtherBodyIndex :type Integer) (bFromSweep :type Boolean) (SweepResult :type "HitResult Structure (by ref)"))
  (if (`self.Open`)
    (`ActorComponent.K2_DestroyComponent` (`self.Door`))
    (else
      (`KismetSystemLibrary.PrintString` "Key required"))))

(fn `UserConstructionScript`)